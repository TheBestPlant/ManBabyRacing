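; Obstacle spawner that periodically drops boulders at random points along a spline.
; On BeginPlay a looping timer fires the spawn event at a fixed interval.
; Each spawn picks a random distance along the spline's length, prints it for debugging, and creates a BP_Boulder at that world location.
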(event `Spawn that Boulder`
  (bind _output_get (set `self.randomFloat` (* (`KismetMathLibrary.RandomFloat`) (`SplineComponent.GetSplineLength` (`self.Spline`)))))
  (`KismetSystemLibrary.PrintString` (`KismetStringLibrary.Conv_DoubleToString` _output_get))
  (`|SpawnActorFromClass` "/Game/_Main/Blueprints/Obstacles/Rock/BP_Boulder.BP_Boulder_C" (`KismetMathLibrary.MakeTransform` (`SplineComponent.GetLocationAtDistanceAlongSpline` (`self.Spline`) _output_get "World")) "Undefined" "MultiplyWithRoot" null null))

(event `self.ReceiveBeginPlay`
  (`KismetSystemLibrary.K2_SetTimerDelegate` (delegate `Spawn that Boulder`) 10.0 true))

(fn `UserConstructionScript`)