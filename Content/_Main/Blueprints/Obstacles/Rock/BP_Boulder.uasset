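; Boulder obstacle that sends players back to their last checkpoint on contact and destroys itself after a fixed lifetime.
; Its sphere overlap checks for the Player tag, skips components tagged "Not Me", then moves the controlled pawn to the location returned by GetLastCheckpointMessage.
; Otherwise, overlapping an actor tagged Die destroys the boulder early.
; No movement logic appears in its graphs.
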(event `self.ReceiveBeginPlay`
  (`KismetSystemLibrary.Delay` 60.0)
  (`self.K2_DestroyActor`))

(event `self.Sphere1.OnComponentBeginOverlap`
  (params (OverlappedComponent :type "PrimitiveComponent Object Reference") (OtherActor :type "Actor Object Reference") (OtherComp :type "PrimitiveComponent Object Reference") (OtherBodyIndex :type Integer) (bFromSweep :type Boolean) (SweepResult :type "HitResult Structure (by ref)"))
  (bind _returnvalue (`Controller.K2_GetPawn` (`self.GetInstigatorController` OtherActor)))
  (if (and (`self.ActorHasTag` OtherActor "Player") (not (`ActorComponent.ComponentHasTag` OtherComp "Not Me")))
    (`KismetSystemLibrary.PrintString` "respawn player")
    (bind _lastcheckpoint (message `/Game/_Main/Blueprints/Interfaces/BPI_Player.GetLastCheckpoint` _returnvalue))
    (`self.K2_SetActorLocation` _returnvalue _lastcheckpoint false false)
    (elif (`self.ActorHasTag` OtherActor "Die")
      (`self.K2_DestroyActor`))))

(fn `UserConstructionScript`)