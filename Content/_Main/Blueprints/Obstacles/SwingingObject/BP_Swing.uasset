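; Swinging obstacle that knocks the player away on contact.
; Two chained timelines pitch RotateThis forward and back at play rates derived from TimeForSwing, restarted by a looping timer every two swing durations.
; Capsule overlaps, except components tagged "Not Me", launch BP_Player away from Cylinder1, then set its ForwardLeft and ForwardRight flags after a short delay.
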(event `SWING`
  (bind _rotatethis (`self.RotateThis`))
  (bind _rotatethis_2 (`self.RotateThis`))
  (bind (_returnvalue_roll _returnvalue_pitch _returnvalue_yaw) (`KismetMathLibrary.BreakRotator` (`SceneComponent.K2_GetComponentRotation` _rotatethis)))
  (bind (_returnvalue_roll_2 _returnvalue_pitch_2 _returnvalue_yaw_2) (`KismetMathLibrary.BreakRotator` (`SceneComponent.K2_GetComponentRotation` _rotatethis_2)))
  (bind (_direction _swing_forward) (`Timeline|SwingForward` :!via `PlayFromStart`)
    (:`Update`
      (`SceneComponent.K2_SetWorldRotation` _rotatethis_2 (`KismetMathLibrary.MakeRotator` _returnvalue_roll_2 _swing_forward _returnvalue_yaw_2) false false))
    (:`Finished`
      (bind (_direction_2 _newtrack_0) (`Timeline|SwingBack` :!via `PlayFromStart`)
        (:`Update`
          (`SceneComponent.K2_SetWorldRotation` _rotatethis (`KismetMathLibrary.MakeRotator` _returnvalue_roll _newtrack_0 _returnvalue_yaw) false false))))))

(event `self.ReceiveBeginPlay`
  (bind _returnvalue (/ 1.0 (`self.TimeForSwing`)))
  (`TimelineComponent.SetPlayRate` (`self.SwingForward`) _returnvalue)
  (`TimelineComponent.SetPlayRate` (`self.SwingBack`) _returnvalue)
  (`self.SWING`)
  (`KismetSystemLibrary.K2_SetTimerDelegate` (delegate `SWING`) (* (`self.TimeForSwing`) 2.0) true))

(event `self.Capsule.OnComponentBeginOverlap`
  (params (OverlappedComponent :type "PrimitiveComponent Object Reference") (OtherActor :type "Actor Object Reference") (OtherComp :type "PrimitiveComponent Object Reference") (OtherBodyIndex :type Integer) (bFromSweep :type Boolean) (SweepResult :type "HitResult Structure (by ref)"))
  (if (not (`ActorComponent.ComponentHasTag` OtherComp "Not Me"))
    (bind _asbp_player (cast `/Game/_Main/Blueprints/Player/BP_Player` OtherActor))
    (bind (_returnvalue_x _returnvalue_y _returnvalue_z) (`KismetMathLibrary.BreakVector` (* (`KismetMathLibrary.Normal` (- (`SceneComponent.K2_GetComponentLocation` (`self.Cylinder1`)) (`self.K2_GetActorLocation` _asbp_player))) -500.0)))
    (`Character.LaunchCharacter` _asbp_player (`KismetMathLibrary.MakeVector` _returnvalue_x _returnvalue_y _returnvalue_z) true true)
    (`KismetSystemLibrary.Delay` 0.2)
    (set `/Game/_Main/Blueprints/Player/BP_Player.ForwardLeft` true _asbp_player)
    (set `/Game/_Main/Blueprints/Player/BP_Player.ForwardRight` true _asbp_player)))

(fn `UserConstructionScript`)