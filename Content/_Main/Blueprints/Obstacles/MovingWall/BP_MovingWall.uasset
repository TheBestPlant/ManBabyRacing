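; BP_MovingWall is an obstacle wall actor meant to move along a referenced spline, starting on BeginPlay.
; A timeline, rate-scaled by the inverse of TimeToComplete, lerps a distance from zero to the spline's length.
; Each update sets actor rotation from the spline's world rotation at that distance, but feeds location from the spline's direction vector rather than its position.
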(event `self.ReceiveBeginPlay`
  (`self.Move Wall`))

(event `Move Wall`
  (bind _spline (`/Game/_Main/Blueprints/Obstacles/MovingWall/BP_WallPath.Spline` (`self.SplineRef`)))
  (`TimelineComponent.SetPlayRate` (`self.T_Move`) (/ 1.0 (`self.TimeToComplete`)))
  (bind (_direction _move_track) (`Timeline|T_Move`)
    (:`Update`
      (bind _returnvalue (`KismetMathLibrary.Lerp` 0.0 (`SplineComponent.GetSplineLength` _spline) _move_track))
      (`self.K2_SetActorLocationAndRotation` (`SplineComponent.GetDirectionAtDistanceAlongSpline` _spline _returnvalue "World") (`SplineComponent.GetRotationAtDistanceAlongSpline` _spline _returnvalue "World")))))

(fn `UserConstructionScript`)