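; BP_Mud is a mud obstacle that increases ground friction and walking braking deceleration for either of two players while inside its Box volume.
; On BeginPlay it caches player characters 0 and 1 as BP_Player references.
; Box overlap events match the actor against those references and write to its CharacterMovement, setting hardcoded lower values on exit rather than restoring saved ones.
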(event `self.ReceiveBeginPlay`
  (bind _asbp_player (cast `/Game/_Main/Blueprints/Player/BP_Player` (`GameplayStatics.GetPlayerCharacter` 0)))
  (set `self.Player1Ref` _asbp_player)
  (bind _asbp_player_2 (cast `/Game/_Main/Blueprints/Player/BP_Player` (`GameplayStatics.GetPlayerCharacter` 1)))
  (set `self.Player2Ref` _asbp_player_2))

(event `self.Box.OnComponentBeginOverlap`
  (params (OverlappedComponent :type "PrimitiveComponent Object Reference") (OtherActor :type "Actor Object Reference") (OtherComp :type "PrimitiveComponent Object Reference") (OtherBodyIndex :type Integer) (bFromSweep :type Boolean) (SweepResult :type "HitResult Structure (by ref)"))
  (bind _charactermovement (`Character.CharacterMovement` (`self.Player2Ref`)))
  (bind _charactermovement_2 (`Character.CharacterMovement` (`self.Player1Ref`)))
  (if (== OtherActor (`self.Player1Ref`))
    (set `CharacterMovementComponent.GroundFriction` 10.0 _charactermovement_2)
    (set `CharacterMovementComponent.BrakingDecelerationWalking` 3000.0 _charactermovement_2)
    (elif (== OtherActor (`self.Player2Ref`))
      (set `CharacterMovementComponent.GroundFriction` 10.0 _charactermovement)
      (set `CharacterMovementComponent.BrakingDecelerationWalking` 3000.0 _charactermovement))))

(event `self.Box.OnComponentEndOverlap`
  (params (OverlappedComponent :type "PrimitiveComponent Object Reference") (OtherActor :type "Actor Object Reference") (OtherComp :type "PrimitiveComponent Object Reference") (OtherBodyIndex :type Integer))
  (bind _charactermovement (`Character.CharacterMovement` (`self.Player1Ref`)))
  (bind _charactermovement_2 (`Character.CharacterMovement` (`self.Player2Ref`)))
  (if (== OtherActor (`self.Player1Ref`))
    (set `CharacterMovementComponent.GroundFriction` 8.0 _charactermovement)
    (set `CharacterMovementComponent.BrakingDecelerationWalking` 2000.0 _charactermovement)
    (elif (== OtherActor (`self.Player2Ref`))
      (set `CharacterMovementComponent.GroundFriction` 8.0 _charactermovement_2)
      (set `CharacterMovementComponent.BrakingDecelerationWalking` 2000.0 _charactermovement_2))))

(fn `UserConstructionScript`)