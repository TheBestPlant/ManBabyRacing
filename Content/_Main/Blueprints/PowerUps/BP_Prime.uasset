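; BP_Prime is a spinning Prime power-up pickup that boosts the player who touches it.
; A looping timer started on BeginPlay advances the actor's yaw to spin it.
; When a Player-tagged actor overlaps the box with a component not tagged "Not Me", it sends ApplyPrimeBoost with a vector built from that actor's forward and up directions, then destroys itself.
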(event `self.ReceiveBeginPlay`
  (`KismetSystemLibrary.K2_SetTimerDelegate` (delegate `Rotate`) 0.01 true))

(event `Rotate`
  (bind (_returnvalue_roll _returnvalue_pitch _returnvalue_yaw) (`KismetMathLibrary.BreakRotator` (`self.K2_GetActorRotation`)))
  (`self.K2_SetActorRotation` (`KismetMathLibrary.MakeRotator` _returnvalue_roll _returnvalue_pitch (mod (+ _returnvalue_yaw 1.0) 360.0))))

(event `self.Box.OnComponentBeginOverlap`
  (params (OverlappedComponent :type "PrimitiveComponent Object Reference") (OtherActor :type "Actor Object Reference") (OtherComp :type "PrimitiveComponent Object Reference") (OtherBodyIndex :type Integer) (bFromSweep :type Boolean) (SweepResult :type "HitResult Structure (by ref)"))
  (if (and (`self.ActorHasTag` OtherActor "Player") (not (`ActorComponent.ComponentHasTag` OtherComp "Not Me")))
    (message `/Game/_Main/Blueprints/Interfaces/BPI_Player.ApplyPrimeBoost` OtherActor (+ (* (`self.GetActorForwardVector` OtherActor) (`self.PrimeForwardBoost`)) (* (`self.GetActorUpVector` OtherActor) (`self.PrimeUpBoost`))))
    (`self.K2_DestroyActor`)))

(fn `UserConstructionScript`
  (`parent.UserConstructionScript`))