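; BP_Feastables is a power-up pickup that gives the player a forward boost on contact.
; A looping timer started on BeginPlay spins the actor around its yaw axis.
; When an actor tagged Player overlaps the box, the pickup sends it a boost message with its forward vector scaled by the configured strength, then destroys itself.
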(event `self.ReceiveBeginPlay`
  (`KismetSystemLibrary.K2_SetTimerDelegate` (delegate `Rotate`) 0.01 true))

(event `Rotate`
  (`self.K2_SetActorRotation` (`KismetMathLibrary.MakeRotator` (.roll (`self.K2_GetActorRotation`)) (.pitch (`self.K2_GetActorRotation`)) (mod (+ (.yaw (`self.K2_GetActorRotation`)) 1.0) 360.0))))

(event `self.Box.OnComponentBeginOverlap`
  (params (OverlappedComponent :type "PrimitiveComponent Object Reference") (OtherActor :type "Actor Object Reference") (OtherComp :type "PrimitiveComponent Object Reference") (OtherBodyIndex :type Integer) (bFromSweep :type Boolean) (SweepResult :type "HitResult Structure (by ref)"))
  (if (`self.ActorHasTag` OtherActor "Player")
    (message `/Game/_Main/Blueprints/Interfaces/BPI_Player.ApplyFeastablesBoost` OtherActor (* (`self.GetActorForwardVector` OtherActor) (`self.FeastiblesForwardBoost`)))
    (`self.K2_DestroyActor`)))

(fn `UserConstructionScript`
  (`parent.UserConstructionScript`))