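; BP_HotDog is a power-up actor that stuns players who touch it, excluding its instigator.
; A box overlap checks the Player tag, sends the stun effect message to that actor, then destroys itself.
; A looping timer started at BeginPlay decrements its remaining life each tick interval, destroying the actor when it runs out.
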(event `Lifetime`
  (bind _returnvalue (`KismetSystemLibrary.K2_SetTimerDelegate` (delegate `Decay`) (`self.LifetimeDecayTickInterval`) true))
  (set `self.DecayTimerHandle` _returnvalue))

(event `self.ReceiveBeginPlay`
  (`parent.ReceiveBeginPlay`)
  (`self.Lifetime`))

(event `Decay`
  (bind _result (`/Engine/EditorBlueprintResources/StandardMacros.DecrementFloat` (`self.CurLife`))
    (:`  `
      (if (<= _result 0.0)
        (`|ExecutionSequence`
          (:`then_0`
            (`KismetSystemLibrary.K2_ClearAndInvalidateTimerHandle` (`self.DecayTimerHandle`)))
          (:`then_1`
            (`/Engine/EditorBlueprintResources/StandardMacros.IsValid` self
              (:`Is Valid`
                (`self.K2_DestroyActor`)))))))))

(event `self.Box.OnComponentBeginOverlap`
  (params (OverlappedComponent :type "PrimitiveComponent Object Reference") (OtherActor :type "Actor Object Reference") (OtherComp :type "PrimitiveComponent Object Reference") (OtherBodyIndex :type Integer) (bFromSweep :type Boolean) (SweepResult :type "HitResult Structure (by ref)"))
  (if (and (`self.ActorHasTag` OtherActor "Player") (!= OtherActor (`self.GetInstigator`)))
    (message `/Game/_Main/Blueprints/Interfaces/BPI_Player.ApplyStunEffect` OtherActor)
    (`self.K2_DestroyActor`)))

(fn `UserConstructionScript`
  (`parent.UserConstructionScript`))