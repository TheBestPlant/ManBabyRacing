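; BP_FinishLineTrigger is the finish line for a two-player race, handling lap counting, the win and the post-race ad.
; On player overlap, it checks the player's checkpoint map against their current lap through message calls, then updates that player's HUD laps.
; At max laps it sets the winner, disables player buttons and requests an ad.
; When the ad media ends, it opens a track-specific powerup shop.
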(event `self.ReceiveBeginPlay`
  (bind _numlapsstart (`self.NumLapsStart`))
  ; Setting OG Values for laps (start at 0 for track 1 but on track 3 you wanna start at 1)
  (`KismetSystemLibrary.Delay` 0.2)
  (bind _foundwidgets (`WidgetBlueprintLibrary.GetAllWidgetsOfClass` "/Game/_Main/Blueprints/Widgets/WBP_HUD.WBP_HUD_C"))
  (bind _output_get (set `self.WBP_HUDRef` (`|GetArrayItem` _foundwidgets)))
  (set `/Game/_Main/Blueprints/Widgets/WBP_HUD.Max Laps` (`self.MaxLaps`) _output_get)
  (set `/Game/_Main/Blueprints/Widgets/WBP_HUD.P1 Laps` _numlapsstart _output_get)
  (set `/Game/_Main/Blueprints/Widgets/WBP_HUD.P2 Laps` _numlapsstart _output_get)
  (`/Game/_Main/Blueprints/Widgets/WBP_HUD.Reset Laps` _output_get))

(event `self.Box.OnComponentBeginOverlap`
  (params (OverlappedComponent :type "PrimitiveComponent Object Reference") (OtherActor :type "Actor Object Reference") (OtherComp :type "PrimitiveComponent Object Reference") (OtherBodyIndex :type Integer) (bFromSweep :type Boolean) (SweepResult :type "HitResult Structure (by ref)"))
  (bind _wbp_hudref (`self.WBP_HUDRef`))
  (bind _wbp_hudref_2 (`self.WBP_HUDRef`))
  (if (and (`self.ActorHasTag` OtherActor "Player") (not (`ActorComponent.ComponentHasTag` OtherComp "Not Me")))
    (`/Engine/EditorBlueprintResources/StandardMacros.DoOnce` false :!label _label
      (:`Completed`
        (bind _curlap (message `/Game/_Main/Blueprints/Interfaces/BPI_Player.GetCurLap` OtherActor))
        (if (< _curlap (`self.MaxLaps`))
          (bind _curlap_2 (message `/Game/_Main/Blueprints/Interfaces/BPI_Player.GetCurLap` OtherActor))
          (bind _checkpointsmap (message `/Game/_Main/Blueprints/Interfaces/BPI_Player.GetCheckpointsMap` OtherActor))
          (bind (_keypin _valuepin) (`|MapForEach` _checkpointsmap)
            (:`then`
              (if (!= (- _valuepin 1) _curlap_2)
                (message `/Game/_Main/Blueprints/Interfaces/BPI_Player.IncrementPassBool` OtherActor false)
                (else
                  (message `/Game/_Main/Blueprints/Interfaces/BPI_Player.IncrementPassBool` OtherActor true))))
            (:`CompletedPin`
              (bind _shouldinc_ (message `/Game/_Main/Blueprints/Interfaces/BPI_Player.IncrementCurLap` OtherActor))
              (if _shouldinc_
                (bind _asplayer_controller (cast `PlayerController` (`self.GetInstigatorController` OtherActor)))
                (if (== _asplayer_controller (`GameplayStatics.GetPlayerController` 0))
                  ; Lap Increase Hud Logic
                  (`/Game/_Main/Blueprints/Widgets/WBP_HUD.P1 Lap Increase` _wbp_hudref)
                  (else
                    (`/Game/_Main/Blueprints/Widgets/WBP_HUD.P2 Lap Increase` _wbp_hudref))))))
          (else
            (if (== OtherActor (`Controller.K2_GetPawn` (`GameplayStatics.GetPlayerController` 0)))
              (set `/Game/_Main/Blueprints/Widgets/WBP_HUD.WinningPlayerNum` 1 (`self.WBP_HUDRef`))
              (else
                (set `/Game/_Main/Blueprints/Widgets/WBP_HUD.WinningPlayerNum` 2 _wbp_hudref_2)))
            (`/Game/_Main/Blueprints/Widgets/WBP_HUD.AskToPlayAd` _wbp_hudref_2)
            (bind _outactors (`GameplayStatics.GetAllActorsOfClass` "/Game/_Main/Blueprints/Player/BP_Player.BP_Player_C"))
            (for _array_element _outactors
              (set `/Game/_Main/Blueprints/Player/BP_Player.bCanPressButtons` false _array_element))))))))

(event `self.Box.OnComponentEndOverlap`
  (params (OverlappedComponent :type "PrimitiveComponent Object Reference") (OtherActor :type "Actor Object Reference") (OtherComp :type "PrimitiveComponent Object Reference") (OtherBodyIndex :type Integer))
  (goto _label :!via `Reset`))

(event `PlayDAAD`
  (bind _admediaplayer (`self.AdMediaPlayer`))
  (`MediaPlayer.OpenSource` _admediaplayer "/Game/_Main/Assets/Ads/GlorpSingsJustTheTwoOfUs.GlorpSingsJustTheTwoOfUs")
  (add `MediaPlayer.OnEndReached` _admediaplayer (delegate `CallFinishAd`)))

(event `CallFinishAd`
  (bind _returnvalue (`GameplayStatics.GetPlayerController` 0))
  (`/Game/_Main/Blueprints/Widgets/WBP_HUD.FinishAd` (`self.WBP_HUDRef`))
  (switch `int` (`self.CurTrack`)
    (:`Default`
      (bind _returnvalue_2 (`|CreateWidget` "/Game/_Main/Blueprints/Widgets/WBP_BuyPowerups.WBP_BuyPowerups_C" _returnvalue :!label _label_2))
      (`UserWidget.AddToViewport` _returnvalue_2 0)
      (`WidgetBlueprintLibrary.SetInputMode_UIOnlyEx` _returnvalue _returnvalue_2))
    (:`1`
      (goto _label_2))
    (:`2`
      (bind _returnvalue_3 (`|CreateWidget` "/Game/_Main/Blueprints/Widgets/WBP_BuyPowerups2.WBP_BuyPowerups2_C" _returnvalue))
      (`UserWidget.AddToViewport` _returnvalue_3 0)
      (`WidgetBlueprintLibrary.SetInputMode_UIOnlyEx` _returnvalue _returnvalue_3)))
  (set `PlayerController.bShowMouseCursor` true _returnvalue))

(fn `UserConstructionScript`)