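; Main menu game mode for ManBabyRacing that is meant to register the two local players with the game instance.
; On BeginPlay it caches GI_ManBabyRacing, then checks that controllers 0 and 1 possess BP_Player pawns.
; Empty Player1 and Player2 slots are assigned their own values rather than the cast pawns, so nothing new is stored.
; Failed casts and already-filled slots only print debug strings.
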(event `self.ReceiveBeginPlay`
  (bind _gi_man_baby_racing (`self.GI Man Baby Racing`))
  (`|ExecutionSequence`
    (:`then_0`
      (bind _asgi_man_baby_racing (cast `/Game/_Main/Blueprints/GI_ManBabyRacing` (`GameplayStatics.GetGameInstance`))
        (:`then`
          (set `self.GI Man Baby Racing` _asgi_man_baby_racing))
        (:`CastFailed`
          (`KismetSystemLibrary.PrintString` "Game Instance cast failed"))))
    (:`then_1`
      (`|ExecutionSequence`
        (:`then_0`
          (cast `/Game/_Main/Blueprints/Player/BP_Player` (`Controller.K2_GetPawn` (`GameplayStatics.GetPlayerController` 0))
            (:`then`
              (bind _player1 (`/Game/_Main/Blueprints/GI_ManBabyRacing.Player1` _gi_man_baby_racing)
                (:`then`
                  (`KismetSystemLibrary.PrintString` "player 1 alr exists"))
                (:`else`
                  (set `/Game/_Main/Blueprints/GI_ManBabyRacing.Player1` _player1 _gi_man_baby_racing))))
            (:`CastFailed`
              (`KismetSystemLibrary.PrintString` "Player 1 cast failed"))))
        (:`then_1`
          (cast `/Game/_Main/Blueprints/Player/BP_Player` (`Controller.K2_GetPawn` (`GameplayStatics.GetPlayerController` 1))
            (:`then`
              (bind _player2 (`/Game/_Main/Blueprints/GI_ManBabyRacing.Player2` _gi_man_baby_racing)
                (:`then`
                  (`KismetSystemLibrary.PrintString` "player 2 alr exists"))
                (:`else`
                  (set `/Game/_Main/Blueprints/GI_ManBabyRacing.Player2` _player2 _gi_man_baby_racing))))
            (:`CastFailed`
              (`KismetSystemLibrary.PrintString` "Player 2 cast failed"))))))))

(fn `UserConstructionScript`)