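; Game mode for the ManBaby racing game that sets up two-player local multiplayer on BeginPlay.
; It creates the second local player if needed and caches that controller and both BP_Player pawns in GI_ManBabyRacing.
; It adds the controller input mapping context for both players, with the mouse-and-keyboard contexts left unconnected.
; Each player gets a WBP_PowerUps widget on their own screen, passed to their pawn as the power-up HUD.
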(event `self.ReceiveBeginPlay`
  (bind _gi_man_baby_racing (`self.GI Man Baby Racing`))
  (`|ExecutionSequence`
    (:`then_0`
      (bind _asgi_man_baby_racing (cast `/Game/_Main/Blueprints/GI_ManBabyRacing` (`GameplayStatics.GetGameInstance`))
        (:`then`
          (bind _output_get (set `self.GI Man Baby Racing` _asgi_man_baby_racing))
          (`/Game/_Main/Blueprints/GI_ManBabyRacing.Player2Controller` _output_get
            (:`then`
              (`KismetSystemLibrary.PrintString` "player 2 alr exists"))
            (:`else`
              (bind _returnvalue (`GameplayStatics.CreatePlayer` 1))
              (set `/Game/_Main/Blueprints/GI_ManBabyRacing.Player2Controller` _returnvalue _asgi_man_baby_racing))))
        (:`CastFailed`
          (`KismetSystemLibrary.PrintString` "Game Instance cast failed"))))
    (:`then_1`
      (`|ExecutionSequence`
        (:`then_0`
          (bind _asbp_player (cast `/Game/_Main/Blueprints/Player/BP_Player` (`Controller.K2_GetPawn` (`GameplayStatics.GetPlayerController` 0)))
            (:`then`
              (`/Game/_Main/Blueprints/GI_ManBabyRacing.Player1` _gi_man_baby_racing
                (:`then`
                  (`KismetSystemLibrary.PrintString` "player 1 alr exists"))
                (:`else`
                  (set `/Game/_Main/Blueprints/GI_ManBabyRacing.Player1` _asbp_player _gi_man_baby_racing))))
            (:`CastFailed`
              (`KismetSystemLibrary.PrintString` "Player 1 cast failed"))))
        (:`then_1`
          (bind _asbp_player_2 (cast `/Game/_Main/Blueprints/Player/BP_Player` (`Controller.K2_GetPawn` (`GameplayStatics.GetPlayerController` 1)))
            (:`then`
              (`/Game/_Main/Blueprints/GI_ManBabyRacing.Player2` _gi_man_baby_racing
                (:`then`
                  (`KismetSystemLibrary.PrintString` "player 2 alr exists"))
                (:`else`
                  (set `/Game/_Main/Blueprints/GI_ManBabyRacing.Player2` _asbp_player_2 _gi_man_baby_racing))))
            (:`CastFailed`
              (`KismetSystemLibrary.PrintString` "Player 2 cast failed"))))))
    (:`then_2`
      ; Set up mapping context for player 1 (MnK) and player 2 (controller)
      (`self.SetUpInputMapping` 0))
    (:`then_3`
      (`self.SetUpInputMapping` 1))
    (:`then_4`
      (bind _returnvalue_2 (`|CreateWidget` "/Game/_Main/Blueprints/Widgets/WBP_PowerUps.WBP_PowerUps_C" (`GameplayStatics.GetPlayerController` 0)))
      (`UserWidget.AddToPlayerScreen` _returnvalue_2 0)
      (`/Game/_Main/Blueprints/Player/BP_Player.SetPowerUpHUD` (`/Game/_Main/Blueprints/GI_ManBabyRacing.Player1` (`self.GI Man Baby Racing`)) _returnvalue_2))
    (:`then_5`
      (bind _returnvalue_3 (`|CreateWidget` "/Game/_Main/Blueprints/Widgets/WBP_PowerUps.WBP_PowerUps_C" (`GameplayStatics.GetPlayerController` 1)))
      (`UserWidget.AddToPlayerScreen` _returnvalue_3 0)
      (`/Game/_Main/Blueprints/Player/BP_Player.SetPowerUpHUD` (`/Game/_Main/Blueprints/GI_ManBabyRacing.Player2` (`self.GI Man Baby Racing`)) _returnvalue_3))))

(fn `SetUpInputMapping`
  (params (ControllerID :type Integer))
  (switch `int` ControllerID
    (:`Default`
      _)
    (:`0`
      _)
    (:`1`
      _))
  (`EnhancedInputSubsystemInterface.AddMappingContext` (pcsubsystem `EnhancedInputLocalPlayerSubsystem` (`GameplayStatics.GetPlayerController` ControllerID)) "/Game/Input/IMC_Controller.IMC_Controller" 0 (struct)))

(fn `UserConstructionScript`)